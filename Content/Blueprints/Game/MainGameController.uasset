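; Main game player controller that handles menus, the end-of-match screen, camera and control mode for the MainGameCharacter.
; On the EvaGameState game-end event, it has MainGameHUD display results and pauses the game.
; Input toggles the menu and cursor, shows frag stats while held, zooms the top-down spring arm and toggles bullet time via global time dilation.
; SetControlMode switches between Mouse and Lua by enabling or disabling the pawn's LuaAgent.
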(event Custom|OnGameEnd
  ;[1 1 1] Game end
  (bind _asmain_game_hud (Utilities|Casting|CastToMainGameHUD (HUD|GetHUD)))
  (Default|DisplayGameResults _asmain_game_hud)
  (Game|SetGamePaused true))

(event EventTick
  (params (DeltaSeconds :type Float%20%28single-precision%29)))

(event EventBeginPlay
  (bind _aseva_game_state (Utilities|Casting|CastToEvaGameState (Game|GetGameState)))
  (Variables|Default|SetGameState _aseva_game_state)
  (EventDispatchers|BindEventtoOnGameEnd _aseva_game_state (delegate Custom|OnGameEnd)))

(event Input|ActionEvents|InputActionShowFrags
  (params (Key :type Key%20Structure :default "AnyKey"))
  ;[1 1 1] Show frag statistics (Shift)
  (:Pressed
    (bind _returnvalue (UserInterface|CreateWidget "/Game/Blueprints/Menu/FragsWidget.FragsWidget_C"))
    (UserInterface|Viewport|AddtoViewport _returnvalue 0))
  (:Released
    (bind _foundwidgets (Widget|GetAllWidgetsOfClass "/Game/Blueprints/Menu/FragsWidget.FragsWidget_C" true))
    (for _array_element _foundwidgets
      (Widget|RemovefromParent _array_element))))

(event Input|MouseEvents|MouseWheelAxis
  (params (AxisValue :type Float%20%28single-precision%29))
  ;[1 1 1] Topdown camera zoom
  (bind _asmain_game_character (Utilities|Casting|CastToMainGameCharacter (Pawn|GetViewTarget)))
  (Variables|/Script/Engine.SpringArmComponent|SetTargetArmLength (Variables|/Game/Blueprints/Game/MainGameCharacter.MainGameCharacter_C|GetSpringArm _asmain_game_character) (Math|Float|Clamp(Float) (- (Variables|/Script/Engine.SpringArmComponent|GetTargetArmLength (Variables|/Game/Blueprints/Game/MainGameCharacter.MainGameCharacter_C|GetSpringArm _asmain_game_character)) (* AxisValue 5e+01)) 3e+02 1e+03)))

(event Input|KeyboardEvents|O
  (params (Key :type Key%20Structure :default "AnyKey"))
  ;[1 1 1] Bullet time
  (:Pressed
    (bind _output_get (Variables|Default|SetBulletTime (not (stale _output_get))))
    (if _output_get
      (Utilities|Time|SetGlobalTimeDilation 0.2)
      (else
        (Utilities|Time|SetGlobalTimeDilation 1.0)))))

(event Input|KeyboardEvents|Tab
  (params (Key :type Key%20Structure :default "AnyKey"))
  ;[1 1 1] Toggle Menu (Tab)
  (:Pressed
    (bind _foundwidgets (Class|WidgetBlueprintLibrary|GetAllWidgetswithInterface "/Game/Blueprints/Menu/MenuInterface.MenuInterface_C" true))
    (if (> (Utilities|Array|Length _foundwidgets) 0)
      (for _array_element _foundwidgets
        (Widget|RemovefromParent _array_element)
        (bind _aseva_game_state (Utilities|Casting|CastToEvaGameState (Game|GetGameState)))
        (bind _returnvalue (Class|EvaGameState|GameFinished _aseva_game_state))
        (if _returnvalue
          _
          (else
            (Game|SetGamePaused false)))
        (Variables|Default|SetCurrentHUD 0)
        (bind _asmain_game_character (Utilities|Casting|CastToMainGameCharacter (Pawn|GetControlledPawn)))
        (bind _returnvalue_2 (Class|EvaCharacter|IsDead _asmain_game_character))
        (if (not _returnvalue_2)
          (Variables|Default|SetbShowMouseCursor false)))
      (else
        (bind _returnvalue_3 (UserInterface|CreateWidget "/Game/Blueprints/Menu/MenuWidget.MenuWidget_C"))
        (UserInterface|Viewport|AddtoViewport _returnvalue_3 0)
        (Variables|Default|SetCurrentHUD _returnvalue_3)
        (Variables|Default|SetbShowMouseCursor true)))))

(fn ConstructionScript)

(fn SetControlMode
  (params (NewMode :type ControllerModeEnum%20Enum))
  (switch Utilities|FlowControl|Switch|SwitchonControllerModeEnum NewMode
    (:NewEnumerator0
      (Variables|Default|SetMode "NewEnumerator0")
      (LocalVariables|SetEnableLuaAgent? false))
    (:NewEnumerator1
      (Variables|Default|SetMode "NewEnumerator1")
      (LocalVariables|SetEnableLuaAgent? true)))
  (bind _asmain_game_character (Utilities|Casting|CastToMainGameCharacter (Pawn|GetControlledPawn)))
  (bind _output_get (Variables|/Script/evaLUAtion2.LuaAgent|SetIsEnabled (Variables|/Game/Blueprints/Game/MainGameCharacter.MainGameCharacter_C|GetLuaAgent _asmain_game_character) (LocalVariables|GetEnableLuaAgent?)))
  (Development|PrintString (Utilities|String|Append "Lua Agent Enabled: " (Utilities|String|ToString(Boolean) _output_get))))