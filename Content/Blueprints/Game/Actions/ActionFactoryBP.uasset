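; ActionFactoryBP is a factory Blueprint that creates action objects from an action type.
; CreateAction switches on the type to pick a class such as ShootAt, ChangeWeapon, Die, Reload or Wait, then constructs and returns an instance with the factory as its outer.
; The Moving type has no dedicated class here and produces a Wait action, the same as Waiting.
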(fn CreateAction
  (params (Type :type EActionType%20Enum))
  (switch Utilities|FlowControl|Switch|SwitchonEActionType Type
    (:Moving
      (LocalVariables|SetKlass "/Game/Blueprints/Game/Actions/Wait.Wait_C"))
    (:Shooting
      (LocalVariables|SetKlass "/Game/Blueprints/Game/Actions/ShootAt.ShootAt_C"))
    (:ChangingWeapon
      (LocalVariables|SetKlass "/Game/Blueprints/Game/Actions/ChangeWeapon.ChangeWeapon_C"))
    (:Dying
      (LocalVariables|SetKlass "/Game/Blueprints/Game/Actions/Die.Die_C"))
    (:Reloading
      (LocalVariables|SetKlass "/Game/Blueprints/Game/Actions/Reload.Reload_C"))
    (:Waiting
      (LocalVariables|SetKlass "/Game/Blueprints/Game/Actions/Wait.Wait_C")))
  (bind _returnvalue (Game|ConstructObjectfromClass (LocalVariables|GetKlass) self))
  (return _returnvalue))