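; Game character driven by an optional Lua agent, acting through a queue of action objects linked by NextAction.
; BeginPlay loads armour, health and ammo from the EvaGameState configuration, attaches the weapon and starts Lua.
; Tick runs the action lifecycle, falling back to Waiting, and asks Lua for decisions when the action is breakable.
; Agent events append actions, all created as Moving, while movement and rotation events act directly.
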(event EventShootatPoint
  (params (vect :type Vector))
  ;[1 1 1] LuaAgent Actions
  (bind _action (CallFunction|CreateAction "Moving"))
  (bind _asshoot_at (Utilities|Casting|CastToShootAt _action))
  (Variables|/Game/Blueprints/Game/Actions/ShootAt.ShootAt_C|Settarget _asshoot_at vect)
  (CallFunction|AddActiontoQueue _action))

(event EventBeginPlay
  (bind _luaagent (Variables|Default|GetLuaAgent))
  ;[1 1 1] Initialization
  (CallFunction|InitializeActor)
  (if (Variables|/Script/evaLUAtion2.LuaAgent|GetIsEnabled _luaagent)
    (Class|LuaAgent|Initialize _luaagent "c:\\ebin.lua")))

(event EventActorBeginOverlap
  (params (OtherActor :type Actor%20Object%20Reference)))

(event EventTick
  (params (DeltaSeconds :type Float%20%28single-precision%29))
  (bind _luaagent (Variables|Default|GetLuaAgent))
  ;[0.5816 1 0.5153] Main Tick Loop
  (Utilities|FlowControl|Sequence
    (:then_0
      ;[1 1 1] odpowiada Actor::Update
      (if (== (Variables|Default|GetcurrentAction) 0)
        (bind _action (CallFunction|CreateAction "Waiting"))
        (bind _output_get (Variables|Default|SetcurrentAction _action))
        (Class|Action|OnEnter _output_get)))
    (:then_1
      (bind _returnvalue (Class|Action|CanExecuteExit (Variables|Default|GetcurrentAction)))
      (if _returnvalue
        (Utilities|FlowControl|Sequence
          (:then_0
            (Class|Action|OnExit (Variables|Default|GetcurrentAction)))
          (:then_1
            (Variables|Default|SetcurrentAction (Variables|/Script/evaLUAtion2.Action|GetnextAction (Variables|Default|GetcurrentAction))))
          (:then_2
            (if (== (Variables|Default|GetcurrentAction) 0)
              (bind _action_2 (CallFunction|CreateAction "Waiting"))
              (Variables|Default|SetcurrentAction _action_2)))
          (:then_3
            (Class|Action|OnEnter (Variables|Default|GetcurrentAction))))))
    (:then_2
      ;[1 1 1] odpowiada Actor::Act
      (if (not (Variables|Default|Getstarted))
        (if (Variables|/Script/evaLUAtion2.LuaAgent|GetIsEnabled _luaagent)
          (Class|LuaAgent|OnStart _luaagent))
        (Variables|Default|Setstarted true)))
    (:then_3
      (if (Variables|/Script/evaLUAtion2.Action|GetIsBreakable (Variables|Default|GetcurrentAction))
        (bind _returnvalue_2 (CallFunction|DecideNextAction))
        (if (!= _returnvalue_2 0)
          (bind _output_get_2 (Variables|Default|SetcurrentAction _returnvalue_2))
          (Class|Action|OnEnter _output_get_2))))))

(event EventReload
  ;[1 1 1] LuaAgent Actions
  (bind _action (CallFunction|CreateAction "Moving"))
  (Utilities|Casting|CastToReload _action)
  (CallFunction|AddActiontoQueue _action))

(event EventWait
  ;[1 1 1] LuaAgent Actions
  (bind _action (CallFunction|CreateAction "Moving"))
  (CallFunction|AddActiontoQueue _action))

(event EventRotate
  (params (rotation :type Rotator))
  ;[1 1 1] BasicActions
  (Transformation|SetActorRotation rotation))

(event EventSelectWeapon
  (params (weapon :type EWeaponType%20Enum :default "Chaingun"))
  ;[1 1 1] LuaAgent Actions
  (bind _action (CallFunction|CreateAction "Moving"))
  (bind _asselect_weapon (Utilities|Casting|CastToSelectWeapon _action))
  (Variables|/Game/Blueprints/Game/Actions/SelectWeapon.SelectWeapon_C|SetWeapon _asselect_weapon "Chaingun")
  (CallFunction|AddActiontoQueue _action))

(event EventMoveDirection
  (params (direction :type Vector))
  ;[1 1 1] BasicActions
  (CallFunction|ActionMoveDirection direction))

(event EventMoveto
  (params (target :type Vector))
  ;[1 1 1] BasicActions
  (CallFunction|ActionMoveto target))

(fn ConstructionScript)

(fn DecideNextAction
  (bind _luaagent (Variables|Default|GetLuaAgent))
  (|CallParentFunction)
  (if (Variables|/Script/evaLUAtion2.LuaAgent|GetIsEnabled _luaagent)
    (Class|LuaAgent|WhattoDo _luaagent)
    (return (Variables|/Script/evaLUAtion2.Action|GetnextAction (Variables|Default|GetcurrentAction)))))

(fn InitializeActor
  (bind _aseva_game_state (Utilities|Casting|CastToEvaGameState (Game|GetGameState))
    (:then
      ;[1 1 1] Set initial destination
      (Variables|Default|Setdestination (Transformation|GetActorLocation))
      (bind _returnvalue (Class|Configuration|GetInt (Variables|/Script/evaLUAtion2.EvaGameState|GetConfiguration _aseva_game_state) "actor.maxArmour"))
      (Variables|Default|Setarmour _returnvalue)
      (bind _returnvalue_2 (Class|Configuration|GetInt (Variables|/Script/evaLUAtion2.EvaGameState|GetConfiguration _aseva_game_state) "actor.maxHealth"))
      (Variables|Default|Sethealth _returnvalue_2)
      (Variables|Default|Setkills 0)
      (Variables|Default|Setkilled 0)
      (Variables|Default|Setfriendkills 0)
      ;[1 1 1] Weapons
      (bind _returnvalue_3 (Class|Configuration|GetInt (Variables|/Script/evaLUAtion2.EvaGameState|GetConfiguration _aseva_game_state) "weapon.Chaingun.Ammo"))
      (bind _returnvalue_4 (Class|Configuration|GetInt (Variables|/Script/evaLUAtion2.EvaGameState|GetConfiguration _aseva_game_state) "weapon.railgun.Ammo"))
      (bind _returnvalue_5 (Class|Configuration|GetInt (Variables|/Script/evaLUAtion2.EvaGameState|GetConfiguration _aseva_game_state) "weapon.rocketlauncher.Ammo"))
      (bind _returnvalue_6 (Class|Configuration|GetInt (Variables|/Script/evaLUAtion2.EvaGameState|GetConfiguration _aseva_game_state) "weapon.Shotgun.Ammo"))
      (Variables|Default|Setloaded (Utilities|Array|MakeArray false false false false))
      (Variables|Default|Setammo (Utilities|Array|MakeArray _returnvalue_3 _returnvalue_4 _returnvalue_5 _returnvalue_6))
      ;[1 1 1] Show weapon
      (Class|SceneComponent|Attachto (Variables|Default|GetHeldWeapon) (Variables|Character|GetMesh) "WeaponPoint" "SnapToTargetIncludingScale" true))
    (:CastFailed
      (Development|PrintString "Failed to cast to EvaGameState")))
  (return))

(fn ActionMoveto
  (params (destination :type Vector))
  (if (> (Math|Vector|VectorLength (- destination (Variables|Default|Getdestination))) 0.05)
    (bind _output_get (Variables|Default|Setdestination destination))
    (AI|Navigation|SimpleMovetoLocation (Pawn|GetController) _output_get))
  (return))

(fn ActionMoveDirection
  (params (B :type Vector))
  ;[1 0.985 0] to w petli i dodaj warunek brzegowy
  (if false
    (bind _output_get (Variables|Default|Setdestination (+ (Variables|Default|Getdestination) B)))
    (AI|Navigation|SimpleMovetoLocation (Pawn|GetController) _output_get))
  (return))

(fn AddActiontoQueue
  (params (nextAction :type Action%20Object%20Reference))
  (Variables|Default|SetLastActionInQueue (Variables|Default|GetcurrentAction))
  (while (!= 0 (Variables|/Script/evaLUAtion2.Action|GetnextAction (Variables|Default|GetLastActionInQueue)))
    (Variables|Default|SetLastActionInQueue (Variables|/Script/evaLUAtion2.Action|GetnextAction (Variables|Default|GetLastActionInQueue))))
  (Variables|/Script/evaLUAtion2.Action|SetnextAction (Variables|Default|GetLastActionInQueue) nextAction)
  (return))