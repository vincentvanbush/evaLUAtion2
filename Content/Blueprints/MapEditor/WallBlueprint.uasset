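; Wall segment actor for the map editor, made of a stretched cube between two end posts, with support for dragging and erasing.
; SetEndingLocations places both posts at floor height, then scales, rotates and centers the cube between them, taking the floor from EvaGameState or the editor controller.
; Cursor events follow the controller's editor state: Idle highlights posts and starts dragging on click, while Erasing tints the wall and removes it on click.
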(event OnBeginCursorOver(CollisionA)
  (params (TouchedComponent :type Primitive%20Component%20Object%20Reference))
  ;[0.9836 0.49 1] Dragging walls
  ;;[1 1 1] wall end cursor over events - highlight cursored-over posts (only in Idle mode)
  (if (Utilities|Enum|Equal(Enum) (Variables|/Game/Blueprints/MapEditor/MapEditorController.MapEditorController_C|GetMapEditorState (Variables|Default|GetControllerRef)) "NewEnumerator0")
    (CallFunction|SetEndsVisibility true)
    (Rendering|Material|SetVectorParameterValue (Variables|Default|GetMaterialA) "Color" "(R=0.939000,G=0.000000,B=0.000000,A=1.000000)" :!class /Script/Engine.MaterialInstanceDynamic)
    (else
      ;[0.2659 0.7049 1] Erasing walls
      (if (Utilities|Enum|Equal(Enum) (Variables|/Game/Blueprints/MapEditor/MapEditorController.MapEditorController_C|GetMapEditorState (Variables|Default|GetControllerRef)) "NewEnumerator4")
        (bind _returnvalue (Rendering|Material|CreateDynamicMaterialInstance "/Game/Environment/Materials/WallCubeMaterial.WallCubeMaterial" :!class /Script/Engine.KismetMaterialLibrary))
        (Rendering|Material|SetVectorParameterValue _returnvalue "Color" "(R=0.570000,G=0.167815,B=0.096763,A=1.000000)" :!class /Script/Engine.MaterialInstanceDynamic)
        (Rendering|Material|SetMaterial (Variables|Default|GetWallCube) 0 _returnvalue)))))

(event OnClicked(CollisionA)
  (params (TouchedComponent :type Primitive%20Component%20Object%20Reference))
  (bind _controllerref (Variables|Default|GetControllerRef))
  (bind _controllerref_2 (Variables|Default|GetControllerRef))
  ;[0.9836 0.49 1] Dragging walls
  ;;[1 1 1] Collision click events - set the Dragging Wall state and set which post is being dragged (also only in Idle mode)
  (if (Utilities|Enum|Equal(Enum) (Variables|/Game/Blueprints/MapEditor/MapEditorController.MapEditorController_C|GetMapEditorState _controllerref_2) "NewEnumerator0")
    (Variables|/Game/Blueprints/MapEditor/MapEditorController.MapEditorController_C|SetDraggedPost _controllerref_2 (Variables|Default|GetCylinderA))
    (CallFunction|SetEditorState "NewEnumerator3")
    (Development|PrintText "OnClicked (Collision)")
    (else
      ;[0.2659 0.7049 1] Erasing walls
      ;;[1 1 1] If in Erasing Wall state, remove the wall when it's clicked
      (if (Utilities|Enum|Equal(Enum) (Variables|/Game/Blueprints/MapEditor/MapEditorController.MapEditorController_C|GetMapEditorState _controllerref) "NewEnumerator4")
        (Utilities|Array|RemoveItem (Variables|/Game/Blueprints/MapEditor/MapEditorController.MapEditorController_C|GetWalls _controllerref) self)
        (Actor|DestroyActor)))))

(event OnClicked(CollisionB)
  (params (TouchedComponent :type Primitive%20Component%20Object%20Reference))
  (bind _controllerref (Variables|Default|GetControllerRef))
  (bind _controllerref_2 (Variables|Default|GetControllerRef))
  ;[0.9836 0.49 1] Dragging walls
  ;;[1 1 1] Collision click events - set the Dragging Wall state and set which post is being dragged (also only in Idle mode)
  (if (Utilities|Enum|Equal(Enum) (Variables|/Game/Blueprints/MapEditor/MapEditorController.MapEditorController_C|GetMapEditorState _controllerref_2) "NewEnumerator0")
    (Variables|/Game/Blueprints/MapEditor/MapEditorController.MapEditorController_C|SetDraggedPost _controllerref_2 (Variables|Default|GetCylinderB))
    (CallFunction|SetEditorState "NewEnumerator3")
    (Development|PrintText "OnClicked (Collision)")
    (else
      ;[0.2659 0.7049 1] Erasing walls
      ;;[1 1 1] If in Erasing Wall state, remove the wall when it's clicked
      (if (Utilities|Enum|Equal(Enum) (Variables|/Game/Blueprints/MapEditor/MapEditorController.MapEditorController_C|GetMapEditorState _controllerref) "NewEnumerator4")
        (Utilities|Array|RemoveItem (Variables|/Game/Blueprints/MapEditor/MapEditorController.MapEditorController_C|GetWalls _controllerref) self)
        (Actor|DestroyActor)))))

(event OnEndCursorOver(CollisionA)
  (params (TouchedComponent :type Primitive%20Component%20Object%20Reference))
  ;[0.9836 0.49 1] Dragging walls
  ;;[1 1 1] wall end cursor over events - highlight cursored-over posts (only in Idle mode)
  (if (Utilities|Enum|Equal(Enum) (Variables|/Game/Blueprints/MapEditor/MapEditorController.MapEditorController_C|GetMapEditorState (Variables|Default|GetControllerRef)) "NewEnumerator0")
    (CallFunction|SetEndsVisibility false)
    (Rendering|Material|SetVectorParameterValue (Variables|Default|GetMaterialA) "Color" "(R=1.000000,G=1.000000,B=1.000000,A=1.000000)" :!class /Script/Engine.MaterialInstanceDynamic)
    (else
      ;[0.2659 0.7049 1] Erasing walls
      (if (Utilities|Enum|Equal(Enum) (Variables|/Game/Blueprints/MapEditor/MapEditorController.MapEditorController_C|GetMapEditorState (Variables|Default|GetControllerRef)) "NewEnumerator4")
        (Rendering|Material|SetMaterial (Variables|Default|GetWallCube) 0 "/Game/Environment/Materials/WallCubeMaterial.WallCubeMaterial")))))

(event OnClicked(WallCube)
  (params (TouchedComponent :type Primitive%20Component%20Object%20Reference))
  (bind _controllerref (Variables|Default|GetControllerRef))
  ;[0.2659 0.7049 1] Erasing walls
  ;;[1 1 1] If in Erasing Wall state, remove the wall when it's clicked
  (if (Utilities|Enum|Equal(Enum) (Variables|/Game/Blueprints/MapEditor/MapEditorController.MapEditorController_C|GetMapEditorState _controllerref) "NewEnumerator4")
    (Utilities|Array|RemoveItem (Variables|/Game/Blueprints/MapEditor/MapEditorController.MapEditorController_C|GetWalls _controllerref) self)
    (Actor|DestroyActor)))

(event OnBeginCursorOver(CollisionB)
  (params (TouchedComponent :type Primitive%20Component%20Object%20Reference))
  ;[0.9836 0.49 1] Dragging walls
  ;;[1 1 1] wall end cursor over events - highlight cursored-over posts (only in Idle mode)
  (if (Utilities|Enum|Equal(Enum) (Variables|/Game/Blueprints/MapEditor/MapEditorController.MapEditorController_C|GetMapEditorState (Variables|Default|GetControllerRef)) "NewEnumerator0")
    (CallFunction|SetEndsVisibility true)
    (Rendering|Material|SetVectorParameterValue (Variables|Default|GetMaterialB) "Color" "(R=0.939000,G=0.000000,B=0.000000,A=1.000000)" :!class /Script/Engine.MaterialInstanceDynamic)
    (else
      ;[0.2659 0.7049 1] Erasing walls
      (if (Utilities|Enum|Equal(Enum) (Variables|/Game/Blueprints/MapEditor/MapEditorController.MapEditorController_C|GetMapEditorState (Variables|Default|GetControllerRef)) "NewEnumerator4")
        (bind _returnvalue (Rendering|Material|CreateDynamicMaterialInstance "/Game/Environment/Materials/WallCubeMaterial.WallCubeMaterial" :!class /Script/Engine.KismetMaterialLibrary))
        (Rendering|Material|SetVectorParameterValue _returnvalue "Color" "(R=0.570000,G=0.167815,B=0.096763,A=1.000000)" :!class /Script/Engine.MaterialInstanceDynamic)
        (Rendering|Material|SetMaterial (Variables|Default|GetWallCube) 0 _returnvalue)))))

(event OnEndCursorOver(CollisionB)
  (params (TouchedComponent :type Primitive%20Component%20Object%20Reference))
  ;[0.9836 0.49 1] Dragging walls
  ;;[1 1 1] wall end cursor over events - highlight cursored-over posts (only in Idle mode)
  (if (Utilities|Enum|Equal(Enum) (Variables|/Game/Blueprints/MapEditor/MapEditorController.MapEditorController_C|GetMapEditorState (Variables|Default|GetControllerRef)) "NewEnumerator0")
    (CallFunction|SetEndsVisibility false)
    (Rendering|Material|SetVectorParameterValue (Variables|Default|GetMaterialB) "Color" "(R=1.000000,G=1.000000,B=1.000000,A=1.000000)" :!class /Script/Engine.MaterialInstanceDynamic)
    (else
      ;[0.2659 0.7049 1] Erasing walls
      (if (Utilities|Enum|Equal(Enum) (Variables|/Game/Blueprints/MapEditor/MapEditorController.MapEditorController_C|GetMapEditorState (Variables|Default|GetControllerRef)) "NewEnumerator4")
        (Rendering|Material|SetMaterial (Variables|Default|GetWallCube) 0 "/Game/Environment/Materials/WallCubeMaterial.WallCubeMaterial")))))

(event OnBeginCursorOver(WallCube)
  (params (TouchedComponent :type Primitive%20Component%20Object%20Reference))
  ;[0.2659 0.7049 1] Erasing walls
  (if (Utilities|Enum|Equal(Enum) (Variables|/Game/Blueprints/MapEditor/MapEditorController.MapEditorController_C|GetMapEditorState (Variables|Default|GetControllerRef)) "NewEnumerator4")
    (bind _returnvalue (Rendering|Material|CreateDynamicMaterialInstance "/Game/Environment/Materials/WallCubeMaterial.WallCubeMaterial" :!class /Script/Engine.KismetMaterialLibrary))
    (Rendering|Material|SetVectorParameterValue _returnvalue "Color" "(R=0.570000,G=0.167815,B=0.096763,A=1.000000)" :!class /Script/Engine.MaterialInstanceDynamic)
    (Rendering|Material|SetMaterial (Variables|Default|GetWallCube) 0 _returnvalue)))

(event OnEndCursorOver(WallCube)
  (params (TouchedComponent :type Primitive%20Component%20Object%20Reference))
  ;[0.2659 0.7049 1] Erasing walls
  (if (Utilities|Enum|Equal(Enum) (Variables|/Game/Blueprints/MapEditor/MapEditorController.MapEditorController_C|GetMapEditorState (Variables|Default|GetControllerRef)) "NewEnumerator4")
    (Rendering|Material|SetMaterial (Variables|Default|GetWallCube) 0 "/Game/Environment/Materials/WallCubeMaterial.WallCubeMaterial")))

(event EventBeginPlay
  (bind _controllerref (CallFunction|GetControllerRef))
  (Variables|Default|SetControllerRef _controllerref))

(event Collision|EventActorBeginOverlap
  (params (OtherActor :type Actor%20Object%20Reference)))

(event EventTick
  (params (DeltaSeconds :type Float%20%28single-precision%29)))

(fn ConstructionScript
  (Utilities|FlowControl|Sequence
    (:then_0
      (bind _returnvalue (Rendering|Material|CreateDynamicMaterialInstance (Variables|Default|GetCylinderA) 0 "/Game/Environment/Materials/WallPostMaterial.WallPostMaterial" :!class /Script/Engine.PrimitiveComponent))
      (Variables|Default|SetMaterialA _returnvalue))
    (:then_1
      (bind _returnvalue_2 (Rendering|Material|CreateDynamicMaterialInstance (Variables|Default|GetCylinderB) 0 "/Game/Environment/Materials/WallPostMaterial.WallPostMaterial" :!class /Script/Engine.PrimitiveComponent))
      (Variables|Default|SetMaterialB _returnvalue_2))))

(fn SetEndingLocations
  (params (BeginXY :type Vector%202D%20Structure) (EndXY :type Vector%202D%20Structure))
  (bind _wallcube (Variables|Default|GetWallCube))
  (bind _returnvalue (Transformation|GetWorldScale _wallcube))
  (bind _aseva_game_state (Utilities|Casting|CastToEvaGameState (Game|GetGameState))
    (:then
      ;[1 1 1] game
      (bind _asfloor (Utilities|Casting|CastToFloor (Variables|/Script/evaLUAtion2.EvaGameState|GetFloorRef _aseva_game_state)))
      (LocalVariables|SetFloorRef _asfloor))
    (:CastFailed
      ;[1 1 1] editor
      (LocalVariables|SetFloorRef (Variables|/Game/Blueprints/MapEditor/MapEditorController.MapEditorController_C|GetFloorRef (Variables|Default|GetControllerRef)))))
  ;[1 1 1] Initialize post location variables
  (bind _output_get (Variables|Default|SetBeginLocation (Math|Vector|MakeVector (.x BeginXY) (.y BeginXY) (.z (Transformation|GetWorldLocation (Variables|/Script/Engine.StaticMeshActor|GetStaticMeshComponent (LocalVariables|GetFloorRef)))))))
  (bind _output_get_2 (Variables|Default|SetEndLocation (Math|Vector|MakeVector (.x EndXY) (.y EndXY) (.z (Transformation|GetWorldLocation (Variables|/Script/Engine.StaticMeshActor|GetStaticMeshComponent (LocalVariables|GetFloorRef)))))))
  ;[1 1 1] Set new locations of wall ends (cylinders)
  (Transformation|SetWorldLocation (Variables|Default|GetCylinderA) _output_get false false)
  (Transformation|SetWorldLocation (Variables|Default|GetCylinderB) _output_get_2 false false)
  ;[1 1 1] Calculate the new length of the wall object
  (Variables|Default|SetEndCylinderDisplacement (- _output_get _output_get_2))
  (bind _output_get_3 (Variables|Default|SetNewWallLength (Math|Vector|VectorLength (- _output_get _output_get_2))))
  ;[1 1 1] Set new WallCube scale according to the calculated length
  (if (>= _output_get_3 0.0)
    (Transformation|SetWorldScale3D _wallcube (Math|Vector|MakeVector (/ _output_get_3 1e+02) (.y _returnvalue) (.z _returnvalue)))
    (else
      (Transformation|SetWorldScale3D _wallcube (Math|Vector|MakeVector (.x _returnvalue) (.y _returnvalue) (.z _returnvalue)))))
  ;[1 1 1] Calculate the angle to rotate the wall
  (Transformation|SetWorldRotation (Variables|Default|GetWallCube) (Math|Conversions|RotationFromXVector (Variables|Default|GetEndCylinderDisplacement)) false false)
  ;[1 1 1] then also rotate the cylinders with the collision zones
  (Transformation|SetWorldRotation (Variables|Default|GetCylinderA) (Math|Conversions|RotationFromXVector (Variables|Default|GetEndCylinderDisplacement)) false false)
  (Transformation|SetWorldRotation (Variables|Default|GetCylinderB) (Math|Conversions|RotationFromXVector (Variables|Default|GetEndCylinderDisplacement)) false false)
  ;[1 1 1] Move the wall between the posts
  (Transformation|SetWorldLocation (Variables|Default|GetWallCube) (/ (+ (Variables|Default|GetBeginLocation) (Variables|Default|GetEndLocation)) 2.0) false false))

(fn SetEndsVisibility
  (params (New%20Ends%20Visible? :type Boolean))
  ;[1 1 1] Sets the visibility of end cylinders
  (bind _output_get (Variables|Default|SetEndsVisible? New%20Ends%20Visible?))
  (Development|SetHiddeninGame (Variables|Default|GetCylinderA) (not _output_get) false)
  (Development|SetHiddeninGame (Variables|Default|GetCylinderB) (not _output_get) false))

(fn SetBeginLocation
  (params (Begin%20XY :type Vector%202D%20Structure))
  (bind _cylinderb (Variables|Default|GetCylinderB))
  (bind _returnvalue (Transformation|GetWorldLocation _cylinderb))
  (CallFunction|SetEndingLocations Begin%20XY (Math|Vector2D|MakeVector2D (.x _returnvalue) (.y _returnvalue))))

(fn SetEndLocation
  (params (End%20XY :type Vector%202D%20Structure))
  (bind _cylindera (Variables|Default|GetCylinderA))
  (bind _returnvalue (Transformation|GetWorldLocation _cylindera))
  (CallFunction|SetEndingLocations (Math|Vector2D|MakeVector2D (.x _returnvalue) (.y _returnvalue)) End%20XY))

(fn GetEndingLocations
  (bind _cylindera (Variables|Default|GetCylinderA))
  (bind _cylinderb (Variables|Default|GetCylinderB))
  (bind _returnvalue (Transformation|GetWorldLocation _cylindera))
  (bind _returnvalue_2 (Transformation|GetWorldLocation _cylinderb))
  (return (Math|Vector2D|MakeVector2D (.x _returnvalue) (.y _returnvalue)) (Math|Vector2D|MakeVector2D (.x _returnvalue_2) (.y _returnvalue_2))))

(fn GetBeginLocation
  (bind _beginlocation (Variables|Default|GetBeginLocation))
  (return (Math|Vector2D|MakeVector2D (.x _beginlocation) (.y _beginlocation))))

(fn GetEndLocation
  (bind _endlocation (Variables|Default|GetEndLocation))
  (return (Math|Vector2D|MakeVector2D (.x _endlocation) (.y _endlocation))))