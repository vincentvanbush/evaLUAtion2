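; Map editor state machine logic that switches and ticks the editing modes held on the MapEditorController, such as wall drawing, dragging, erasing, powerup and waypoint placement.
; SetEditorState applies each mode's entry effects, toggling the placeholder wall, mouse events and powerup placeholder.
; StateTick moves the active wall ends or placeholder to the controller's snapped cursor coordinates.
; When dragging, the grabbed post's component name decides which wall end moves.
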(fn SetEditorState
  (params (NewState :type MapEditorStateEnum%20Enum))
  ;[1 1 1] Set controller reference
  (bind _controllerref (CallFunction|GetControllerRef))
  (LocalVariables|SetControllerRef _controllerref)
  (switch Utilities|FlowControl|Switch|SwitchonMapEditorStateEnum NewState
    (:NewEnumerator0
      ;[1 1 1] Idle state
      (Variables|/Game/Blueprints/MapEditor/MapEditorController.MapEditorController_C|SetMapEditorState (LocalVariables|GetControllerRef) "NewEnumerator0")
      (CallFunction|HidePlaceholderWall)
      (CallFunction|DestroyPowerupPlaceholder))
    (:NewEnumerator1
      ;[1 1 1] Drawing Wall Start state
      (Variables|/Game/Blueprints/MapEditor/MapEditorController.MapEditorController_C|SetIsDrawing? (LocalVariables|GetControllerRef) true)
      (Variables|/Game/Blueprints/MapEditor/MapEditorController.MapEditorController_C|SetMapEditorState (LocalVariables|GetControllerRef) "NewEnumerator1")
      (Rendering|SetActorHiddenInGame (Variables|/Game/Blueprints/MapEditor/MapEditorController.MapEditorController_C|GetDrawingWallBlueprintRef (LocalVariables|GetControllerRef)) false)
      (Default|SetEndsVisibility (Variables|/Game/Blueprints/MapEditor/MapEditorController.MapEditorController_C|GetDrawingWallBlueprintRef (LocalVariables|GetControllerRef)) true)
      (Variables|/Script/Engine.PlayerController|SetbEnableMouseOverEvents (LocalVariables|GetControllerRef) false)
      (Variables|/Script/Engine.PlayerController|SetbEnableClickEvents (LocalVariables|GetControllerRef) false)
      (CallFunction|DestroyPowerupPlaceholder))
    (:NewEnumerator2
      ;[1 1 1] Drawing Wall End state
      (Variables|/Game/Blueprints/MapEditor/MapEditorController.MapEditorController_C|SetMapEditorState (LocalVariables|GetControllerRef) "NewEnumerator2"))
    (:NewEnumerator3
      ;[1 1 1] Dragging Wall state
      (Variables|/Game/Blueprints/MapEditor/MapEditorController.MapEditorController_C|SetMapEditorState (LocalVariables|GetControllerRef) "NewEnumerator3")
      (Variables|/Script/Engine.PlayerController|SetbEnableMouseOverEvents (LocalVariables|GetControllerRef) false))
    (:NewEnumerator4
      ;[1 1 1] Erasing Wall state
      (Variables|/Game/Blueprints/MapEditor/MapEditorController.MapEditorController_C|SetMapEditorState (LocalVariables|GetControllerRef) "NewEnumerator4")
      (CallFunction|HidePlaceholderWall)
      (CallFunction|DestroyPowerupPlaceholder))
    (:NewEnumerator5
      ;[1 1 1] Drawing Powerups state
      (Variables|/Game/Blueprints/MapEditor/MapEditorController.MapEditorController_C|SetMapEditorState (LocalVariables|GetControllerRef) "NewEnumerator5")
      (CallFunction|HidePlaceholderWall))
    (:NewEnumerator6
      ;[1 1 1] Drawing Waypoints state
      (Variables|/Game/Blueprints/MapEditor/MapEditorController.MapEditorController_C|SetMapEditorState (LocalVariables|GetControllerRef) "NewEnumerator6")
      (CallFunction|HidePlaceholderWall))))

(fn StateTick
  ;[1 1 1] Set controller reference
  (bind _controllerref (CallFunction|GetControllerRef))
  (bind _output_get (LocalVariables|SetController%20Ref _controllerref))
  ;[1 1 1] Then, depending on current Editor State...
  (switch Utilities|FlowControl|Switch|SwitchonMapEditorStateEnum (Variables|/Game/Blueprints/MapEditor/MapEditorController.MapEditorController_C|GetMapEditorState _output_get)
    (:NewEnumerator1
      ;[1 1 1] In Drawing Wall Start state...
      ;;[1 1 1] Drag both start and end
      (Default|SetEndingLocations (Variables|/Game/Blueprints/MapEditor/MapEditorController.MapEditorController_C|GetDrawingWallBlueprintRef (LocalVariables|GetController%20Ref)) (Variables|/Game/Blueprints/MapEditor/MapEditorController.MapEditorController_C|GetSnap%20Coords (LocalVariables|GetController%20Ref)) (Variables|/Game/Blueprints/MapEditor/MapEditorController.MapEditorController_C|GetSnap%20Coords (LocalVariables|GetController%20Ref))))
    (:NewEnumerator2
      ;[1 1 1] In Drawing Wall End state...
      ;;[1 1 1] Leave start unchanged, move end only
      (Default|SetEndingLocations (Variables|/Game/Blueprints/MapEditor/MapEditorController.MapEditorController_C|GetDrawingWallBlueprintRef (LocalVariables|GetController%20Ref)) (Math|Vector2D|MakeVector2D (.x (Transformation|GetWorldLocation (Variables|/Game/Blueprints/MapEditor/WallBlueprint.WallBlueprint_C|GetCylinderA (Variables|/Game/Blueprints/MapEditor/MapEditorController.MapEditorController_C|GetDrawingWallBlueprintRef (LocalVariables|GetController%20Ref))))) (.y (Transformation|GetWorldLocation (Variables|/Game/Blueprints/MapEditor/WallBlueprint.WallBlueprint_C|GetCylinderA (Variables|/Game/Blueprints/MapEditor/MapEditorController.MapEditorController_C|GetDrawingWallBlueprintRef (LocalVariables|GetController%20Ref)))))) (Variables|/Game/Blueprints/MapEditor/MapEditorController.MapEditorController_C|GetSnap%20Coords (LocalVariables|GetController%20Ref))))
    (:NewEnumerator3
      ;[1 1 1] In Dragging Wall state...
      (bind _aswall_blueprint (Utilities|Casting|CastToWallBlueprint (Components|GetOwner (Variables|/Game/Blueprints/MapEditor/MapEditorController.MapEditorController_C|GetDraggedPost (LocalVariables|GetController%20Ref)))))
      (bind _output_get_2 (Variables|/Game/Blueprints/MapEditor/MapEditorController.MapEditorController_C|SetDragged%20Wall (LocalVariables|GetController%20Ref) _aswall_blueprint))
      (if (Utilities|Enum|Equal(Enum) (Utilities|GetObjectName (Variables|/Game/Blueprints/MapEditor/MapEditorController.MapEditorController_C|GetDraggedPost (LocalVariables|GetController%20Ref))) "CylinderA")
        (Default|SetBeginLocation _output_get_2 (Variables|/Game/Blueprints/MapEditor/MapEditorController.MapEditorController_C|GetSnap%20Coords (LocalVariables|GetController%20Ref)))
        (else
          (Default|SetEndLocation _output_get_2 (Variables|/Game/Blueprints/MapEditor/MapEditorController.MapEditorController_C|GetSnap%20Coords (LocalVariables|GetController%20Ref))))))
    (:NewEnumerator5
      ;[1 1 1] In Drawing Powerups state...
      (Transformation|SetActorLocation (Variables|/Game/Blueprints/MapEditor/MapEditorController.MapEditorController_C|GetPowerupPlaceholderRef (LocalVariables|GetController%20Ref)) (Math|Vector|MakeVector (.x (Variables|/Game/Blueprints/MapEditor/MapEditorController.MapEditorController_C|GetSnap%20Coords (LocalVariables|GetController%20Ref))) (.y (Variables|/Game/Blueprints/MapEditor/MapEditorController.MapEditorController_C|GetSnap%20Coords (LocalVariables|GetController%20Ref))) 0.0) false false :!label _label))
    (:NewEnumerator6
      (goto _label))))

(fn GetControllerRef
  (bind _asmap_editor_controller (Utilities|Casting|CastToMapEditorController (Game|GetPlayerController 0))
    (:then
      _)
    (:CastFailed
      _))
  (return _asmap_editor_controller))

(fn HidePlaceholderWall
  (bind _controllerref (CallFunction|GetControllerRef))
  (LocalVariables|SetControllerRef _controllerref)
  (Rendering|SetActorHiddenInGame (Variables|/Game/Blueprints/MapEditor/MapEditorController.MapEditorController_C|GetDrawingWallBlueprintRef (LocalVariables|GetControllerRef)) true)
  (Variables|/Script/Engine.PlayerController|SetbEnableMouseOverEvents (LocalVariables|GetControllerRef) true)
  (Variables|/Script/Engine.PlayerController|SetbEnableClickEvents (LocalVariables|GetControllerRef) true)
  (return))

(fn DestroyPowerupPlaceholder
  (bind _controllerref (CallFunction|GetControllerRef))
  (if (not (== (Variables|/Game/Blueprints/MapEditor/MapEditorController.MapEditorController_C|GetPowerupPlaceholderRef _controllerref) 0))
    (Actor|DestroyActor (Variables|/Game/Blueprints/MapEditor/MapEditorController.MapEditorController_C|GetPowerupPlaceholderRef _controllerref))))