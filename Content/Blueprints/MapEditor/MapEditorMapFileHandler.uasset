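; Map editor handler that saves and loads map layouts as .emf files through the controller's file handler.
; Saving gathers floor size, wall endpoints and powerup positions with types, converting units by a factor of ten.
; Loading reverses the scaling, resizes the floor and spawns walls with hidden ends, appending them to the controller's list without clearing it.
; SpawnPowerups handles only types 6 to 9, all currently spawning a Railgun.
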(fn SaveMapObjects
  (params (Filename :type String))
  (if (Utilities|String|EndsWith Filename ".emf")
    (LocalVariables|SetMapFilename Filename)
    (else
      (LocalVariables|SetMapFilename (Utilities|String|Append Filename ".emf"))))
  (bind _controllerref (CallFunction|GetControllerRef))
  (LocalVariables|SetControllerRef _controllerref)
  ;[1 1 1] Creating array of walls to save
  (for _array_element (Variables|/Game/Blueprints/MapEditor/MapEditorController.MapEditorController_C|GetWalls (LocalVariables|GetControllerRef))
    (bind (_wallbegin _wallend) (Default|GetEndingLocations _array_element))
    (bind _output_get (LocalVariables|SetWallCoord (Utilities|Struct|MakeVector2Dpair (/ _wallbegin 1e+01) (/ _wallend 1e+01))))
    (Utilities|Array|Add (LocalVariables|GetWallsCoords) _output_get))
  ;[1 1 1] creating array of powerups to save
  (for _array_element_2 (Variables|/Game/Blueprints/MapEditor/MapEditorController.MapEditorController_C|GetPowerups (LocalVariables|GetControllerRef))
    (bind _output_get_2 (LocalVariables|SetPowerupCoord (Utilities|Struct|MakePowerupInfo (Math|Vector2D|MakeVector2D (/ (.x (Transformation|GetActorLocation _array_element_2)) 1e+01) (/ (.y (Transformation|GetActorLocation _array_element_2)) 1e+01)) (Variables|/Game/Blueprints/Powerups/Powerup.Powerup_C|GetPowerupType _array_element_2))))
    (Utilities|Array|Add (LocalVariables|GetPowerupsCoords) _output_get_2))
  ;[1 1 1] saving to file
  (bind (_sizex _sizey) (Default|GetMapSize (Variables|/Game/Blueprints/MapEditor/MapEditorController.MapEditorController_C|GetFloorRef (LocalVariables|GetControllerRef))))
  (bind _returnvalue (Class|MapFileHandler|SaveMapFile (Variables|/Game/Blueprints/MapEditor/MapEditorController.MapEditorController_C|GetFileHandlerRef (LocalVariables|GetControllerRef)) (LocalVariables|GetMapFilename) (Utilities|Array|MakeArray (* _sizex 10) (* _sizey 10)) (LocalVariables|GetWallsCoords) (LocalVariables|GetPowerupsCoords)))
  (if _returnvalue
    (Development|PrintString 0 "zapisano")
    (else
      (Development|PrintString 0 "nie zapisano"))))

(fn LoadMapObjects
  (params (Filename :type String))
  (bind _controllerref (CallFunction|GetControllerRef))
  (bind _output_get (LocalVariables|SetControllerRef _controllerref))
  (if (Utilities|String|EndsWith Filename ".emf")
    (LocalVariables|SetMap%20Filename Filename)
    (else
      (LocalVariables|SetMap%20Filename (Utilities|String|Append Filename ".emf"))))
  (bind (_mapsize _waypointscoords _wallscoords _powerupscoords) (Class|MapFileHandler|LoadMapFile (Variables|/Game/Blueprints/MapEditor/MapEditorController.MapEditorController_C|GetFileHandlerRef _output_get) (LocalVariables|GetMap%20Filename)))
  (LocalVariables|SetWalls%20Coords _wallscoords)
  (LocalVariables|SetPowerups%20Coords _powerupscoords)
  ;[1 1 1] setting map size according to values from file
  (Default|SetMapSize (Variables|/Game/Blueprints/MapEditor/MapEditorController.MapEditorController_C|GetFloorRef (LocalVariables|GetControllerRef)) (/ (Utilities|Array|Get(acopy) _mapsize) 10) (/ (Utilities|Array|Get(acopy) _mapsize 1) 10))
  ;[1 1 1] spawning walls objects
  (for _array_element (LocalVariables|GetWalls%20Coords)
    (bind _returnvalue (Game|SpawnActorfromClass "/Game/Blueprints/MapEditor/WallBlueprint.WallBlueprint_C" (Math|Transform|MakeTransform "0.0,0.0,0.0" "0, 0, 0" "1,1,1") "Undefined" 0 0))
    (Default|SetEndingLocations _returnvalue (* (.acoord _array_element) 1e+01) (* (.bcoord _array_element) 1e+01))
    (Utilities|Array|Add (Variables|/Game/Blueprints/MapEditor/MapEditorController.MapEditorController_C|GetWalls (LocalVariables|GetControllerRef)) _returnvalue)
    (Default|SetEndsVisibility _returnvalue false))
  (CallFunction|SpawnPowerups (LocalVariables|GetPowerups%20Coords)))

(fn SpawnPowerups
  (params (PowerupsCoords :type Array%20of%20Powerup%20Info%20Structures))
  (bind _controllerref (CallFunction|GetControllerRef))
  (LocalVariables|SetControllerRef _controllerref)
  (for _array_element PowerupsCoords
    (LocalVariables|SetPowerupCoords (.coord _array_element))
    (switch int (.type _array_element)
      (:6
        (bind _returnvalue (Game|SpawnActorfromClass "/Game/Blueprints/Powerups/Railgun.Railgun_C" (Math|Transform|MakeTransform "0, 0, 0" "0, 0, 0" "1,1,1") "Undefined" 0 0))
        (bind _returnvalue_2 (Utilities|Array|Add (Variables|/Game/Blueprints/MapEditor/MapEditorController.MapEditorController_C|GetPowerups (LocalVariables|GetControllerRef)) _returnvalue))
        (LocalVariables|SetCurrentPowerupIndex _returnvalue_2))
      (:7
        (bind _returnvalue_3 (Game|SpawnActorfromClass "/Game/Blueprints/Powerups/Railgun.Railgun_C" (Math|Transform|MakeTransform "0, 0, 0" "0, 0, 0" "1,1,1") "Undefined" 0 0))
        (bind _returnvalue_4 (Utilities|Array|Add (Variables|/Game/Blueprints/MapEditor/MapEditorController.MapEditorController_C|GetPowerups (LocalVariables|GetControllerRef)) _returnvalue_3))
        (LocalVariables|SetCurrentPowerupIndex _returnvalue_4))
      (:8
        (bind _returnvalue_5 (Game|SpawnActorfromClass "/Game/Blueprints/Powerups/Railgun.Railgun_C" (Math|Transform|MakeTransform "0, 0, 0" "0, 0, 0" "1,1,1") "Undefined" 0 0))
        (bind _returnvalue_6 (Utilities|Array|Add (Variables|/Game/Blueprints/MapEditor/MapEditorController.MapEditorController_C|GetPowerups (LocalVariables|GetControllerRef)) _returnvalue_5))
        (LocalVariables|SetCurrentPowerupIndex _returnvalue_6))
      (:9
        (bind _returnvalue_7 (Game|SpawnActorfromClass "/Game/Blueprints/Powerups/Railgun.Railgun_C" (Math|Transform|MakeTransform "0, 0, 0" "0, 0, 0" "1,1,1") "Undefined" 0 0))
        (bind _returnvalue_8 (Utilities|Array|Add (Variables|/Game/Blueprints/MapEditor/MapEditorController.MapEditorController_C|GetPowerups (LocalVariables|GetControllerRef)) _returnvalue_7))
        (LocalVariables|SetCurrentPowerupIndex _returnvalue_8)))
    (Transformation|SetWorldLocation (Variables|/Script/Engine.StaticMeshActor|GetStaticMeshComponent (Utilities|Array|Get(acopy) (Variables|/Game/Blueprints/MapEditor/MapEditorController.MapEditorController_C|GetPowerups (LocalVariables|GetControllerRef)) (LocalVariables|GetCurrentPowerupIndex))) (Math|Vector|MakeVector (.x (* (LocalVariables|GetPowerupCoords) 1e+01)) (.y (* (LocalVariables|GetPowerupCoords) 1e+01)) 0.0) false false)))