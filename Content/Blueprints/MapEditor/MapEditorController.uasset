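; Map editor controller that lets the user draw walls on the floor with the mouse, toggled from MapEditorWidget.
; While drawing, Tick traces under the cursor and moves the preview wall's ends to the point from WhereToSnap.
; Left clicks fix the start, then commit the wall to Walls and spawn the next.
; WhereToSnap rounds to the grid in floor-corner coordinates, optionally overriding with nearby existing wall endpoints.
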(event Custom|Draw%20Wall%20Clicked
  (params (IsClicked? :type Boolean))
  (bind _drawingwallblueprintref (Variables|Default|GetDrawingWallBlueprintRef))
  ;[1 1 1] Events for setting the editor state (triggered in MapEditorWidget)
  ;;[1 1 1] User clicks the 'draw walls' button - entering Drawing Wall Start state (Drawing Wall End handled elsewhere)
  (if IsClicked?
    (Variables|Default|SetIsDrawingWall? true)
    (Variables|Default|SetMapEditorState "NewEnumerator1")
    (Rendering|SetActorHiddenInGame _drawingwallblueprintref false)
    (Default|SetEndsVisibility _drawingwallblueprintref true)
    (Variables|Default|SetbEnableMouseOverEvents false)
    (Variables|Default|SetbEnableClickEvents false)
    (else
      (Variables|Default|SetMapEditorState "NewEnumerator0")
      (Rendering|SetActorHiddenInGame true)
      (Variables|Default|SetbEnableMouseOverEvents true)
      (Variables|Default|SetbEnableClickEvents true))))

(event EventBeginPlay
  (Variables|Default|SetbEnableMouseOverEvents true))

(event EventTick
  (params (DeltaSeconds :type Float%20%28single-precision%29))
  (bind (_locationx _locationy) (Game|Player|GetMousePosition))
  (bind _drawingwallblueprintref (Variables|Default|GetDrawingWallBlueprintRef))
  (bind (_worldlocation _worlddirection) (Class|PlayerController|DeprojectScreenPositiontoWorld _locationx _locationy))
  (bind _cylindera (Variables|/Game/Blueprints/MapEditor/WallBlueprint.WallBlueprint_C|GetCylinderA _drawingwallblueprintref))
  (bind _returnvalue (Transformation|GetWorldLocation _cylindera))
  ;[1 1 1] This section is responsible for 'painting' on the surface
  ;;[1 1 1] Tracing the cursor and casting it onto the surface
  (if (Variables|Default|GetIsDrawingWall?)
    (Variables|Default|SetTraceLineStart _worldlocation)
    (Variables|Default|SetMouseDirection _worlddirection)
    (Variables|Default|SetTraceLineEnd (+ (Variables|Default|GetTraceLineStart) (* (Variables|Default|GetMouseDirection) 5e+03)))
    (bind (_outhit _returnvalue_2) (Collision|LineTraceByChannel (Variables|Default|GetTraceLineStart) (Variables|Default|GetTraceLineEnd) "TraceTypeQuery1" false (Utilities|Array|MakeArray (Variables|Default|GetDrawingWallBlueprintRef)) "None" false))
    ;;[1 1 1] only if actually traced something
    (bind _output_get (Variables|Default|SetTraced? _returnvalue_2))
    (if _output_get
      (Utilities|FlowControl|Sequence
        (:then_0
          ;;[0 0.06502 1] TODO: See the WhereToSnap function, the magic shall belong there.
          (bind _snapto (CallFunction|WheretoSnap (Math|Vector2D|MakeVector2D (.x (.impactpoint _outhit)) (.y (.impactpoint _outhit)))))
          (Variables|Default|SetSnap%20Coords _snapto))
        (:then_1
          ;;[1 1 1] Then, depending on current Editor State...
          (switch Utilities|FlowControl|Switch|SwitchonMapEditorStateEnum (Variables|Default|GetMapEditorState)
            (:NewEnumerator1
              ;[1 1 1] In Drawing Wall Start state...
              ;;[1 1 1] Drag both start and end
              (Default|SetEndingLocations (Variables|Default|GetDrawingWallBlueprintRef) (Variables|Default|GetSnap%20Coords) (Variables|Default|GetSnap%20Coords)))
            (:NewEnumerator2
              ;[1 1 1] In Drawing Wall End state...
              ;;[1 1 1] Leave start unchanged, move end only
              (Default|SetEndingLocations _drawingwallblueprintref (Math|Vector2D|MakeVector2D (.x _returnvalue) (.y _returnvalue)) (Variables|Default|GetSnap%20Coords)))))))))

(event Input|MouseEvents|LeftMouseButton
  (params (Key :type Key%20Structure :default "AnyKey"))
  ;[0 0.02342 1] TODO: Handle the following scenario:
  ;;[1 0.9707 0.09264] this is unfinished but thats about how it should work - try this out :)
  (:Pressed
    (if (Variables|Default|GetTraced?)
      (switch Utilities|FlowControl|Switch|SwitchonMapEditorStateEnum (Variables|Default|GetMapEditorState)
        (:NewEnumerator1
          (Variables|Default|SetMapEditorState "NewEnumerator2"))
        (:NewEnumerator2
          (Utilities|Array|AddUnique (Variables|Default|GetWalls) (Variables|Default|GetDrawingWallBlueprintRef))
          (Variables|/Game/Blueprints/MapEditor/WallBlueprint.WallBlueprint_C|SetCursorOverEventsEnabled? (Variables|Default|GetDrawingWallBlueprintRef) true)
          (Default|SetEndsVisibility (Variables|Default|GetDrawingWallBlueprintRef) false)
          (bind _returnvalue (Game|SpawnActorfromClass "/Game/Blueprints/MapEditor/WallBlueprint.WallBlueprint_C" (Math|Transform|MakeTransform "0.000000, 0, 0" "0, 0, 0" "1,1,1") "AlwaysSpawn" 0 0))
          (bind _output_get (Variables|Default|SetDrawingWallBlueprintRef _returnvalue))
          (Default|SetEndsVisibility _output_get true)
          (Variables|Default|SetMapEditorState "NewEnumerator1"))))))

(fn ConstructionScript)

(fn WheretoSnap
  (params (SnapFrom :type Vector%202D%20Structure))
  (bind _gridscale (Variables|Default|GetGridScale))
  (bind _returnvalue (Math|Float|Truncate _gridscale))
  (bind _returnvalue_2 (Math|Float|Truncate _gridscale))
  ;[0 0.01481 0.85] Snap To Grid Calculations
  (Utilities|FlowControl|Sequence
    (:then_0
      ;;[1 1 1] Move positions to +/+ coords in 3D space
      (bind (_sizex _sizey) (Default|GetMapSize (Variables|Default|GetFloorRef)))
      (Utilities|FlowControl|Sequence
        (:then_0
          (LocalVariables|SetMapXHalf (Math|Conversions|ToFloat(Integer) (/ (* _sizex 100) 2))))
        (:then_1
          (LocalVariables|SetMapYHalf (Math|Conversions|ToFloat(Integer) (/ (* _sizey 100) 2))))
        (:then_2
          (bind _output_get (LocalVariables|SetAbsXPos (+ (.x SnapFrom) (Math|Conversions|ToFloat(Integer) (/ (* _sizex 100) 2)))))
          (LocalVariables|SetSnapX (Math|Float|Truncate _output_get)))
        (:then_3
          (bind _output_get_2 (LocalVariables|SetAbsYPos (+ (.y SnapFrom) (Math|Conversions|ToFloat(Integer) (/ (* _sizey 100) 2)))))
          (LocalVariables|SetSnapY (Math|Float|Truncate _output_get_2)))))
    (:then_1
      ;;[1 1 1] Check Snap To Grid
      (if (Variables|Default|GetSnapToGrid?)
        ;;[1 1 1] Snap To Grid
        (Utilities|FlowControl|Sequence
          (:then_0
            ;;;[1 1 1] Get new X position
            (if (>= (.Remainder (Math|Float|Division(WholeandRemainder) (LocalVariables|GetAbsXPos) _gridscale)) (/ _gridscale 2.0))
              (LocalVariables|SetSnapX (+ (* (.ReturnValue (Math|Float|Division(WholeandRemainder) (LocalVariables|GetAbsXPos) _gridscale)) _returnvalue_2) _returnvalue_2))
              (else
                (LocalVariables|SetSnapX (* (.ReturnValue (Math|Float|Division(WholeandRemainder) (LocalVariables|GetAbsXPos) _gridscale)) _returnvalue_2)))))
          (:then_1
            ;;;[1 1 1] Get new Y position
            (if (>= (.Remainder (Math|Float|Division(WholeandRemainder) (LocalVariables|GetAbsYPos) _gridscale)) (/ _gridscale 2.0))
              (LocalVariables|SetSnapY (+ (* (.ReturnValue (Math|Float|Division(WholeandRemainder) (LocalVariables|GetAbsYPos) _gridscale)) _returnvalue) _returnvalue))
              (else
                (LocalVariables|SetSnapY (* (.ReturnValue (Math|Float|Division(WholeandRemainder) (LocalVariables|GetAbsYPos) _gridscale)) _returnvalue))))))))
    (:then_2
      ;;[1 1 1] Check Snap To Walls
      (if (Variables|Default|GetSnapToWalls?)
        ;;[1 1 1] Snap To Walls
        (bind _array_element (Utilities|Array|ForEachLoopwithBreak (Variables|Default|GetWalls))
          (:LoopBody
            (Utilities|FlowControl|Sequence
              (:then_0
                (bind _output_get_3 (LocalVariables|SetElementDistX (Math|Float|Sqrt (+ (Math|Float|Square (Math|Float|Absolute(Float) (- (+ (.x (Variables|/Game/Blueprints/MapEditor/WallBlueprint.WallBlueprint_C|GetBeginLocation _array_element)) (LocalVariables|GetMapXHalf)) (LocalVariables|GetAbsXPos)))) (Math|Float|Square (Math|Float|Absolute(Float) (- (+ (.y (Variables|/Game/Blueprints/MapEditor/WallBlueprint.WallBlueprint_C|GetBeginLocation _array_element)) (LocalVariables|GetMapYHalf)) (LocalVariables|GetAbsYPos)))))))))
              (:then_1
                (bind _output_get_4 (LocalVariables|SetElementDistY (Math|Float|Sqrt (+ (Math|Float|Square (Math|Float|Absolute(Float) (- (+ (.x (Variables|/Game/Blueprints/MapEditor/WallBlueprint.WallBlueprint_C|GetEndLocation _array_element)) (LocalVariables|GetMapXHalf)) (LocalVariables|GetAbsXPos)))) (Math|Float|Square (Math|Float|Absolute(Float) (- (+ (.y (Variables|/Game/Blueprints/MapEditor/WallBlueprint.WallBlueprint_C|GetEndLocation _array_element)) (LocalVariables|GetMapYHalf)) (LocalVariables|GetAbsYPos)))))))))
              (:then_2
                (if (>= (LocalVariables|GetElementDistY) (LocalVariables|GetElementDistX))
                  (if (>= (LocalVariables|GetBestElement) (LocalVariables|GetElementDistX))
                    (LocalVariables|SetSnapX (Math|Float|Truncate (+ (.x (Variables|/Game/Blueprints/MapEditor/WallBlueprint.WallBlueprint_C|GetBeginLocation _array_element)) (LocalVariables|GetMapXHalf))))
                    (LocalVariables|SetSnapY (Math|Float|Truncate (+ (.y (Variables|/Game/Blueprints/MapEditor/WallBlueprint.WallBlueprint_C|GetBeginLocation _array_element)) (LocalVariables|GetMapYHalf))))
                    (LocalVariables|SetBestElement _output_get_3))
                  (elif (>= (LocalVariables|GetBestElement) (LocalVariables|GetElementDistY))
                    (LocalVariables|SetSnapX (Math|Float|Truncate (+ (.x (Variables|/Game/Blueprints/MapEditor/WallBlueprint.WallBlueprint_C|GetEndLocation _array_element)) (LocalVariables|GetMapXHalf))))
                    (LocalVariables|SetSnapY (Math|Float|Truncate (+ (.y (Variables|/Game/Blueprints/MapEditor/WallBlueprint.WallBlueprint_C|GetEndLocation _array_element)) (LocalVariables|GetMapYHalf))))
                    (LocalVariables|SetBestElement _output_get_4)))))))))
    (:then_3
      ;;[1 1 1] Return results
      (return (Math|Vector2D|MakeVector2D (- (Math|Conversions|ToFloat(Integer) (LocalVariables|GetSnapX)) (LocalVariables|GetMapXHalf)) (- (Math|Conversions|ToFloat(Integer) (LocalVariables|GetSnapY)) (LocalVariables|GetMapYHalf)))))))