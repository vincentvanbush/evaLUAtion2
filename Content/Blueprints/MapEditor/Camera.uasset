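; Map editor camera pawn or actor that registers itself with MapEditorController as the editor camera and becomes the view target on begin play.
; Each tick it moves the root along stored forward and right axis input, rotated by the root's yaw so movement follows the view.
; Zoom inputs step the spring arm length, kept above zero, and holding right mouse turns the actor's yaw.
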(event EventBeginPlay
  ;[1 1 1] Setting up camera
  (Input|EnableInput (Game|GetPlayerController 0))
  (bind _asmap_editor_controller (Utilities|Casting|CastToMapEditorController (Game|GetPlayerController 0))
    (:then
      (bind _output_get (Variables|/Game/Blueprints/MapEditor/MapEditorController.MapEditorController_C|SetEditorCamera _asmap_editor_controller self))
      (Game|Player|SetViewTargetwithBlend _asmap_editor_controller _output_get 0.0 "VTBlend_Linear" 0.0 false))
    (:CastFailed
      _))
  (Variables|Default|SetArmLength (Variables|/Script/Engine.SpringArmComponent|GetTargetArmLength (Variables|Default|GetCameraBoom))))

(event EventTick
  (params (DeltaSeconds :type Float%20%28single-precision%29))
  (bind _mainroot (Variables|Default|GetMainRoot))
  ;[1 1 1] Moving camera with WSAD
  (bind _output_get (Variables|Default|SetCameraDisplacement (Math|Vector|MakeVector (Variables|Default|GetForwardAxis) (Variables|Default|GetRightAxis) 0.0)))
  (bind _output_get_2 (Variables|Default|SetCameraDisplacement (Math|Vector|RotateVector _output_get (Math|Rotator|MakeRotator 0.0 0.0 (.Yaw (Math|Rotator|BreakRotator (Transformation|GetWorldRotation _mainroot)))))))
  (Transformation|SetWorldLocation (Variables|Default|GetMainRoot) (+ (* _output_get_2 (Variables|Default|GetCameraSpeed)) (Transformation|GetWorldLocation _mainroot)) false false))

(event Input|ActionEvents|InputActionZoomIn
  (params (Key :type Key%20Structure :default "AnyKey"))
  ;[1 1 1] Zoom in
  ;;[1 1 1] Scroll up
  (:Pressed
    (if (> (- (Variables|Default|GetArmLength) (Variables|Default|GetZoomSpeed)) 0.0)
      (bind _output_get (Variables|Default|SetArmLength (- (Variables|Default|GetArmLength) (Variables|Default|GetZoomSpeed))))
      (Variables|/Script/Engine.SpringArmComponent|SetTargetArmLength (Variables|Default|GetCameraBoom) _output_get))))

(event Input|ActionEvents|InputActionZoomOut
  (params (Key :type Key%20Structure :default "AnyKey"))
  ;[1 1 1] Zoom out
  ;;[1 1 1] Scrool down
  (:Pressed
    (bind _output_get (Variables|Default|SetArmLength (+ (Variables|Default|GetArmLength) (Variables|Default|GetZoomSpeed))))
    (Variables|/Script/Engine.SpringArmComponent|SetTargetArmLength (Variables|Default|GetCameraBoom) _output_get)))

(event Input|AxisEvents|InputAxisCameraForward
  (params (AxisValue :type Float%20%28single-precision%29))
  (Variables|Default|SetForwardAxis AxisValue))

(event Input|AxisEvents|InputAxisCameraRight
  (params (AxisValue :type Float%20%28single-precision%29))
  (Variables|Default|SetRightAxis AxisValue))

(event Input|AxisEvents|InputAxisTurn
  (params (AxisValue :type Float%20%28single-precision%29))
  (bind _returnvalue (Transformation|GetActorRotation))
  (if (Game|Player|IsInputKeyDown (Game|GetPlayerController 0) "RightMouseButton")
    (Transformation|SetActorRotation (Math|Rotator|MakeRotator (.roll _returnvalue) (.pitch _returnvalue) (+ (.yaw _returnvalue) (* AxisValue (Variables|Default|GetRotationSpeed)))))))

(fn ConstructionScript)