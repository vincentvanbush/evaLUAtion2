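; Resizable map floor actor, shared by the map editor and the main game, whose X/Y scale encodes the map size.
; SetMapSize rescales it in 100-unit cells and recenters it so one corner stays at the world origin.
; Outside MainGameMode, it also has the MapEditorController refresh the grid texture, then removes that controller's walls, powerups and waypoints lying beyond the new bounds.
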(event EventBeginPlay
  (bind _asmap_editor_controller (Utilities|Casting|CastToMapEditorController (Game|GetPlayerController 0)))
  (Variables|Default|SetControllerRef _asmap_editor_controller))

(event Collision|EventActorBeginOverlap
  (params (OtherActor :type Actor%20Object%20Reference)))

(event EventTick
  (params (DeltaSeconds :type Float%20%28single-precision%29)))

(fn ConstructionScript
  (Variables|Default|SetSizeX 1e+01)
  (Variables|Default|SetSizeY 1e+01))

(fn SetMapSize
  (params (NewSizeX :type Float%20%28single-precision%29) (NewSizeY :type Float%20%28single-precision%29))
  (bind _returnvalue (Transformation|GetActorTransform))
  (bind _output_get (Variables|Default|SetSizeX NewSizeX))
  (bind _output_get_2 (Variables|Default|SetSizeY NewSizeY))
  (Transformation|SetActorTransform (Math|Transform|MakeTransform (Math|Vector|MakeVector (* (/ NewSizeX 2.0) 1e+02) (* (/ NewSizeY 2.0) 1e+02) (.z (.location _returnvalue))) (.rotation _returnvalue) (Math|Vector|MakeVector _output_get _output_get_2 (.z (.scale _returnvalue)))))
  ;[1 1 1] we needn't set grid and truncate objects during the game (editor only stuff)
  (Utilities|Casting|CastToMainGameMode (Game|GetGameMode)
    (:CastFailed
      (Default|SetGridTexture (Variables|Default|GetControllerRef))
      (CallFunction|TruncateObjects))))

(fn GetMapSize
  (bind _returnvalue (Class|Actor|GetActorRelativeScale3D))
  (return (Math|Float|Truncate (.x _returnvalue)) (Math|Float|Truncate (.y _returnvalue))))

(fn TruncateObjects
  (bind _sizex (Variables|Default|GetSizeX))
  (bind _sizey (Variables|Default|GetSizeY))
  (bind _wallstotruncate (Variables|Default|GetWallsToTruncate))
  (bind _controllerref (Variables|Default|GetControllerRef))
  (bind _returnvalue (* _sizex 1e+02))
  (bind _returnvalue_2 (* _sizey 1e+02))
  ;[1 1 1] determine which walls to truncate
  (for _array_element (Variables|/Game/Blueprints/MapEditor/MapEditorController.MapEditorController_C|GetWalls (Variables|Default|GetControllerRef))
    (bind (_wallbegin _wallend) (Default|GetEndingLocations _array_element))
    (if (Math|Boolean|ORBoolean (> (.x _wallbegin) _returnvalue) (> (.y _wallbegin) _returnvalue_2) (> (.x _wallend) _returnvalue) (> (.y _wallend) _returnvalue_2))
      (Actor|DestroyActor _array_element)
      (Utilities|Array|AddUnique (Variables|Default|GetWallsToTruncate) _array_element)))
  ;[1 1 1] truncate walls
  (for _array_element_2 _wallstotruncate
    (Utilities|Array|RemoveItem (Variables|/Game/Blueprints/MapEditor/MapEditorController.MapEditorController_C|GetWalls (Variables|Default|GetControllerRef)) _array_element_2))
  (Utilities|Array|Clear _wallstotruncate)
  ;[1 1 1] determine which powerups to truncate
  (bind _output_get (Variables|Default|SetPowerupsToTruncate (Variables|/Game/Blueprints/MapEditor/MapEditorController.MapEditorController_C|GetPowerups _controllerref)))
  (Utilities|Array|AppendArray _output_get (Variables|/Game/Blueprints/MapEditor/MapEditorController.MapEditorController_C|GetWaypoints _controllerref))
  (for _array_element_3 _output_get
    (if (or (> (.x (.location (Transformation|GetActorTransform _array_element_3))) (* (Variables|Default|GetSizeX) 1e+02)) (> (.y (.location (Transformation|GetActorTransform _array_element_3))) (* (Variables|Default|GetSizeY) 1e+02)))
      (Default|RemovePowerup _array_element_3))))