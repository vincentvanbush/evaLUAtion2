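; Powerup actor that can be removed in the map editor and reports its type through GetPowerupType.
; Hovering the cursor over its Sphere sets the Color parameter on its materials to red, then back to black on exit.
; Clicking it in one specific map editor state removes it from the controller's Powerups array and destroys it.
; SetHighlight and the construction script are empty.
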(event OnBeginCursorOver(Sphere)
  (params (TouchedComponent :type Primitive%20Component%20Object%20Reference))
  ;[1 1 1] Highlight when removing
  (for _array_element (Variables|Default|GetMaterials)
    (Rendering|Material|SetVectorParameterValue _array_element "Color" "(R=1.000000,G=0.000000,B=0.000000,A=1.000000)" :!class /Script/Engine.MaterialInstanceDynamic)))

(event OnClicked(Sphere)
  (params (TouchedComponent :type Primitive%20Component%20Object%20Reference))
  (bind _self self)
  ;[1 1 1] Remove Powerup when clicked
  (bind _controllerref (CallFunction|GetControllerRef))
  (if (Utilities|Enum|Equal(Enum) (Variables|/Game/Blueprints/MapEditor/MapEditorController.MapEditorController_C|GetMapEditorState _controllerref) "NewEnumerator7")
    (if (not (== (Utilities|Array|FindItem (Variables|/Game/Blueprints/MapEditor/MapEditorController.MapEditorController_C|GetPowerups _controllerref) _self) -1))
      (Utilities|Array|RemoveItem (Variables|/Game/Blueprints/MapEditor/MapEditorController.MapEditorController_C|GetPowerups _controllerref) _self)
      (Actor|DestroyActor))))

(event OnEndCursorOver(Sphere)
  (params (TouchedComponent :type Primitive%20Component%20Object%20Reference))
  ;[1 1 1] Highlight when removing
  (for _array_element (Variables|Default|GetMaterials)
    (Rendering|Material|SetVectorParameterValue _array_element "Color" "(R=0.000000,G=0.000000,B=0.000000,A=1.000000)" :!class /Script/Engine.MaterialInstanceDynamic)))

(fn ConstructionScript)

(fn SetHighlight
  (params (IsHighlighted :type Boolean)))

(fn GetPowerupType
  (return (Variables|Default|GetPowerupType)))