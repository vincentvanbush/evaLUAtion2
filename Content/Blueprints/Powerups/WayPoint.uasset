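; WayPoint is a waypoint actor, filed with the powerups, that reveals its connections when the cursor hovers over it.
; Cursor-over events on its Sphere tell the controller to show or hide the waypoint connections, passing itself as the waypoint.
; After running the parent construction script, it creates a dynamic emissive material instance on the powerup mesh and stores it in a Materials array.
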(event OnBeginCursorOver(Sphere)
  (params (TouchedComponent :type Primitive%20Component%20Object%20Reference))
  (bind _controllerref (CallFunction|GetControllerRef))
  (Default|ToggleWaypointConnectionsVisibility _controllerref true self))

(event OnEndCursorOver(Sphere)
  (params (TouchedComponent :type Primitive%20Component%20Object%20Reference))
  (bind _controllerref (CallFunction|GetControllerRef))
  (Default|ToggleWaypointConnectionsVisibility _controllerref false self))

(event EventBeginPlay)

(event EventActorBeginOverlap
  (params (OtherActor :type Actor%20Object%20Reference)))

(event EventTick
  (params (DeltaSeconds :type Float%20%28single-precision%29)))

(fn ConstructionScript
  (|CallParentFunction)
  (Utilities|FlowControl|Sequence
    (:then_0
      (bind _returnvalue (Rendering|Material|CreateDynamicMaterialInstance (Variables|Default|GetPowerupStaticMesh) 0 "/Game/Environment/Materials/WallAssets/Simple_emmisive2.Simple_emmisive2" :!class /Script/Engine.PrimitiveComponent))
      (Utilities|Array|Add (Variables|Default|GetMaterials) _returnvalue))))